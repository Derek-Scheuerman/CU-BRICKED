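; Dice rack that spawns a 3x3 grid of BP_RackSlot actors and scores it five seconds after BeginPlay.
; CalculateRack gathers each row and column, runs a hand-written Shell sort, and keeps each line's highest value or expression result.
; Symbol dice apply their operation to both neighbours through ExpressionSetUp and RunExpression.
; It returns summed row and column scores, spawning a value-driven particle burst over each positive slot.
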(event EventBeginPlay
  (for _index (range 0 2)
    (for _index_2 (range 0 2)
      (bind _returnvalue (Game|SpawnActorfromClass "/Game/Coding/Rack/BP_RackSlot.BP_RackSlot_C" (Math|Transform|MakeTransform (Math|Vector|MakeVector (Math|Conversions|ToFloat(Integer) (* _index 500)) (Math|Conversions|ToFloat(Integer) (* (- _index_2 1) 500)) 0.0) "0, 0, 0" "1.000000,1.000000,1.000000") "Undefined" "MultiplyWithRoot" 0 _index_2 _index 0))
      (Utilities|Array|Add (Variables|Default|GetRackView) _returnvalue)))
  (Utilities|FlowControl|Delay 5.0)
  (CallFunction|CalculateRack))

(fn ConstructionScript)

(fn CalculateRack
  (bind _currrackseries (LocalVariables|GetCurrRackSeries))
  (bind _currrackseries_2 (LocalVariables|GetCurrRackSeries))
  (Utilities|FlowControl|Sequence
    (:then_0
      ;[0.15 0.15 0.15 0.5] Row Scoring
      (Utilities|Array|Clear (Variables|Default|GetRowTotals))
      (for _index (range 0 (- (Variables|Default|GetRow) 1))
        (LocalVariables|SetLocRowCount _index)
        (Utilities|Array|Clear (LocalVariables|GetCurrRackSeries))
        (Utilities|Array|Add (Variables|Default|GetRowTotals) 0)
        (for _array_element (Variables|Default|GetRackView)
          (if (== (Variables|/Game/Coding/Rack/BP_RackSlot.BP_RackSlot_C|GetRow _array_element) (LocalVariables|GetLocRowCount))
            (Utilities|Array|Add _currrackseries_2 _array_element)))
        (bind _organizedarray (CallFunction|ShellSort _currrackseries_2 true))
        (for (_array_element_2 _array_index) _organizedarray
          (if (.symbol (Variables|/Game/Coding/Rack/BP_RackSlot.BP_RackSlot_C|GetDiceData _array_element_2))
            (bind _returnvalue (CallFunction|ExpressionSetUp (.operation (Variables|/Game/Coding/Rack/BP_RackSlot.BP_RackSlot_C|GetDiceData _array_element_2)) (LocalVariables|GetCurrRackSeries) _array_index))
            (if (> _returnvalue (Utilities|Array|Get(acopy) (Variables|Default|GetRowTotals) (LocalVariables|GetLocRowCount)))
              (Utilities|Array|SetArrayElem (Variables|Default|GetRowTotals) (LocalVariables|GetLocRowCount) _returnvalue))
            (elif (> (.value (Variables|/Game/Coding/Rack/BP_RackSlot.BP_RackSlot_C|GetDiceData _array_element_2)) (Utilities|Array|Get(acopy) (Variables|Default|GetRowTotals) (LocalVariables|GetLocRowCount)))
              (Utilities|Array|SetArrayElem (Variables|Default|GetRowTotals) (LocalVariables|GetLocRowCount) (.value (Variables|/Game/Coding/Rack/BP_RackSlot.BP_RackSlot_C|GetDiceData _array_element_2))))))))
    (:then_1
      ;[0.15 0.15 0.15 0.5] Column Scoring
      (Utilities|Array|Clear (Variables|Default|GetColTotals))
      (for _index_2 (range 0 (- (Variables|Default|GetColumn) 1))
        (LocalVariables|SetLocColCount _index_2)
        (Utilities|Array|Clear (LocalVariables|GetCurrRackSeries))
        (Utilities|Array|Add (Variables|Default|GetColTotals) 0)
        (for _array_element_3 (Variables|Default|GetRackView)
          (if (== (Variables|/Game/Coding/Rack/BP_RackSlot.BP_RackSlot_C|GetColumn _array_element_3) (LocalVariables|GetLocColCount))
            (Utilities|Array|Add _currrackseries _array_element_3)))
        (bind _organizedarray_2 (CallFunction|ShellSort _currrackseries false))
        (for (_array_element_4 _array_index_2) _organizedarray_2
          (if (.symbol (Variables|/Game/Coding/Rack/BP_RackSlot.BP_RackSlot_C|GetDiceData _array_element_4))
            (bind _returnvalue_2 (CallFunction|ExpressionSetUp (.operation (Variables|/Game/Coding/Rack/BP_RackSlot.BP_RackSlot_C|GetDiceData _array_element_4)) (LocalVariables|GetCurrRackSeries) _array_index_2))
            (if (> _returnvalue_2 (Utilities|Array|Get(acopy) (Variables|Default|GetColTotals) (LocalVariables|GetLocColCount)))
              (Utilities|Array|SetArrayElem (Variables|Default|GetColTotals) (LocalVariables|GetLocColCount) _returnvalue_2))
            (elif (> (.value (Variables|/Game/Coding/Rack/BP_RackSlot.BP_RackSlot_C|GetDiceData _array_element_4)) (Utilities|Array|Get(acopy) (Variables|Default|GetColTotals) (LocalVariables|GetLocColCount)))
              (Utilities|Array|SetArrayElem (Variables|Default|GetColTotals) (LocalVariables|GetLocColCount) (.value (Variables|/Game/Coding/Rack/BP_RackSlot.BP_RackSlot_C|GetDiceData _array_element_4))))))))
    (:then_2
      ;[0.15 0.15 0.15 0.5] Calculate Total Scores
      (for _array_element_5 (Variables|Default|GetRowTotals)
        (LocalVariables|SetRowScore (+ _array_element_5 (LocalVariables|GetRowScore))))
      (for _array_element_6 (Variables|Default|GetColTotals)
        (LocalVariables|SetColumnScore (+ _array_element_6 (LocalVariables|GetColumnScore))))
      ;[0.15 0.15 0.15 0.5] VFX check value of slot and spawn that many particals
      (for _array_element_7 (Variables|Default|GetRackView)
        (if (> (.value (Variables|/Game/Coding/Rack/BP_RackSlot.BP_RackSlot_C|GetDiceData _array_element_7)) 0)
          (bind _returnvalue_3 (Niagara|SpawnSystematLocation "/Game/VFX/TestBurst.TestBurst" (+ (Transformation|GetActorLocation _array_element_7) "0.000000,0.000000,150.000000")))
          (Class|NiagaraComponent|SetVariableInt _returnvalue_3 "User.Boris" (.value (Variables|/Game/Coding/Rack/BP_RackSlot.BP_RackSlot_C|GetDiceData _array_element_7)))))
      (return (LocalVariables|GetRowScore) (LocalVariables|GetColumnScore)))))

(fn ShellSort
  (params (UnorganizedArray :type Array%20of%20BP%20Rack%20Slot%20Object%20References) (Row? :type Boolean))
  (bind _output_get (LocalVariables|SetSize (Utilities|Array|Length UnorganizedArray)))
  (LocalVariables|SetS (/ _output_get 2))
  (while (> (LocalVariables|GetS) 0)
    (for _index (range (LocalVariables|GetS) (- (LocalVariables|GetSize) 1))
      (bind _output_get_2 (LocalVariables|SetJ (- _index (LocalVariables|GetS))))
      (while (and (>= _output_get_2 0) (> (Math|Integer|SelectInt (Variables|/Game/Coding/Rack/BP_RackSlot.BP_RackSlot_C|GetRow (Utilities|Array|Get(acopy) UnorganizedArray (Math|Integer|Absolute(Integer) (LocalVariables|GetJ)))) (Variables|/Game/Coding/Rack/BP_RackSlot.BP_RackSlot_C|GetColumn (Utilities|Array|Get(acopy) UnorganizedArray (Math|Integer|Absolute(Integer) (LocalVariables|GetJ)))) Row?) (Math|Integer|SelectInt (Variables|/Game/Coding/Rack/BP_RackSlot.BP_RackSlot_C|GetRow (Utilities|Array|Get(acopy) UnorganizedArray (+ (LocalVariables|GetJ) (LocalVariables|GetS)))) (Variables|/Game/Coding/Rack/BP_RackSlot.BP_RackSlot_C|GetColumn (Utilities|Array|Get(acopy) UnorganizedArray (+ (LocalVariables|GetJ) (LocalVariables|GetS)))) Row?)))
        (Utilities|Array|Swap UnorganizedArray (LocalVariables|GetJ) (+ (LocalVariables|GetJ) (LocalVariables|GetS)))
        (LocalVariables|SetJ (- (LocalVariables|GetJ) (LocalVariables|GetS)))))
    (LocalVariables|SetS (/ (LocalVariables|GetS) 2)))
  (return UnorganizedArray))

(fn ExpressionSetUp
  (params (Symbol :type E_Symbols%20Enum :default "NewEnumerator0") (CurrSeries :type Array%20of%20BP%20Rack%20Slot%20Object%20References) (SymbolIndex :type Integer))
  (bind _returnvalue (- SymbolIndex 1))
  (bind _returnvalue_2 (+ SymbolIndex 1))
  (bind _output (Utilities|Array|Get(acopy) CurrSeries _returnvalue_2))
  (bind _output_2 (Utilities|Array|Get(acopy) CurrSeries _returnvalue))
  (bind _dicedata (Variables|/Game/Coding/Rack/BP_RackSlot.BP_RackSlot_C|GetDiceData _output))
  (bind _dicedata_2 (Variables|/Game/Coding/Rack/BP_RackSlot.BP_RackSlot_C|GetDiceData _output_2))
  (bind _value (Utilities|Struct|BreakDiceSide_Struct _dicedata))
  (bind _value_2 (Utilities|Struct|BreakDiceSide_Struct _dicedata_2))
  (bind (_add _sub _mult _div _exp) (CallFunction|RunExpression _value_2 _value))
  (bind _returnvalue_3 (Utilities|Select :Index Symbol :NewEnumerator0 _add :NewEnumerator1 _sub :NewEnumerator2 _mult :NewEnumerator3 _div :NewEnumerator4 _exp :NewEnumerator5 0))
  (if (and (Utilities|Array|IsValidIndex CurrSeries _returnvalue) (Utilities|Array|IsValidIndex CurrSeries _returnvalue_2))
    (Development|PrintText (Utilities|Text|FormatText "{O}: {R}" (|GenerictoText Symbol) _returnvalue_3))
    (return _returnvalue_3)))

(fn RunExpression
  (params (A :type Integer) (B :type Integer))
  (return (+ A B) (- A B) (* A B) (/ A B) (Math|Float|Truncate (Math|Float|Power (Math|Conversions|ToFloat(Integer) A) (Math|Conversions|ToFloat(Integer) B)))))