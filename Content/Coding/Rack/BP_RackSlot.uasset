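; BP_RackSlot is a single rack slot at a row and column that tracks the die resting in it.
; On begin play it shows its row and column as text and passes each of its four compass-side W_RackAddition widgets its world location.
; The DiceCheck overlap volume stores an entering die and its up-side data unless the stored die still overlaps, and resets both once that die no longer overlaps.
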(event OnComponentBeginOverlap(DiceCheck)
  (params (OverlappedComponent :type Primitive%20Component%20Object%20Reference) (OtherActor :type Actor%20Object%20Reference) (OtherComp :type Primitive%20Component%20Object%20Reference) (OtherBodyIndex :type Integer) (bFromSweep :type Boolean) (SweepResult :type Hit%20Result%20Structure%20%28by%20ref%29))
  (if (not (Collision|IsOverlappingActor (Variables|Default|GetDiceCheck) (Variables|Default|GetDie) :!class /Script/Engine.PrimitiveComponent))
    (Variables|Default|SetDie OtherActor)
    (bind _asbp_dice (Utilities|Casting|CastToBP_Dice OtherActor))
    (Variables|Default|SetDiceData (Variables|/Game/Dice/BP_Dice.BP_Dice_C|GetUpSideData _asbp_dice))))

(event OnComponentEndOverlap(DiceCheck)
  (params (OverlappedComponent :type Primitive%20Component%20Object%20Reference) (OtherActor :type Actor%20Object%20Reference) (OtherComp :type Primitive%20Component%20Object%20Reference) (OtherBodyIndex :type Integer))
  (if (not (Collision|IsOverlappingActor (Variables|Default|GetDiceCheck) (Variables|Default|GetDie) :!class /Script/Engine.PrimitiveComponent))
    (Variables|Default|SetDiceData (Utilities|Struct|MakeDiceSide_Struct false 0 "NewEnumerator0"))
    (Variables|Default|SetDie 0)))

(event EventBeginPlay
  (Rendering|Components|TextRender|SetText (Variables|Default|GetTextRender) (Utilities|Text|FormatText "{R} {C}" (Variables|Default|GetRow) (Variables|Default|GetColumn)))
  (CallFunction|SetWidgetData (Variables|Default|GetNorthWidget))
  (CallFunction|SetWidgetData (Variables|Default|GetEastWidget))
  (CallFunction|SetWidgetData (Variables|Default|GetSouthWidget))
  (CallFunction|SetWidgetData (Variables|Default|GetWestWidget)))

(fn ConstructionScript)

(fn SetWidgetData
  (params (Target :type Widget%20Component%20Object%20Reference))
  (bind _asw_rack_addition (Utilities|Casting|CastToW_RackAddition (UserInterface|GetWidget Target)))
  (Variables|/Game/Widgets/W_RackAddition.W_RackAddition_C|SetWorldLoc _asw_rack_addition (Transformation|GetWorldLocation Target)))